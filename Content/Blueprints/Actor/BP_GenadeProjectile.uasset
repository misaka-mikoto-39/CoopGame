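; Grenade projectile actor that explodes on hit or one second after BeginPlay, whichever comes first, then destroys itself.
; The Explode event spawns the explosion particle effect and applies radial damage at the actor's location, credited to the instigator controller.
; It also draws a temporary debug sphere showing the damage radius.
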(event Custom|Explode
  (bind _returnvalue (Transformation|GetActorLocation))
  (bind _damageradius (Variables|Default|GetDamageRadius))
  (Effects|SpawnEmitteratLocation "/Game/WeaponEffects/Explosion/P_Explosion.P_Explosion" _returnvalue)
  (Game|Damage|ApplyRadialDamage 1e+02 _returnvalue _damageradius 0 0 self (Game|GetInstigatorController) false "ECC_Visibility")
  (Rendering|Debug|DrawDebugSphere _returnvalue _damageradius 12 "(R=0.248561,G=1.000000,B=0.000000,A=1.000000)" 2.0 2.0))

(event Collision|EventHit
  (params (MyComp :type Primitive%20Component%20Object%20Reference) (Other :type Actor%20Object%20Reference) (OtherComp :type Primitive%20Component%20Object%20Reference) (bSelfMoved :type Boolean) (HitLocation :type Vector :default "0, 0, 0") (HitNormal :type Vector :default "0, 0, 0") (NormalImpulse :type Vector :default "0, 0, 0") (Hit :type Hit%20Result%20Structure%20%28by%20ref%29))
  (CallFunction|Explode)
  (Actor|DestroyActor))

(event EventBeginPlay
  (Utilities|FlowControl|Delay 1.0)
  (CallFunction|Explode)
  (Actor|DestroyActor))

(fn ConstructionScript)