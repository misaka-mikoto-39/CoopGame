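; BP_SuperSpeed is a power-up that temporarily makes the activating actor walk ten times faster.
; On activation it stores the actor and sets its CharacterMovementComponent's MaxWalkSpeed to ten times GetMaxSpeed.
; On expiry, if the stored actor is still valid, it divides GetMaxSpeed by the same factor, then calls the parent's expiry logic.
; Both changes derive from the current mode-dependent max speed rather than a cached original walk speed.
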(event EventOnExpired
  (bind _activate_for (Variables|Default|GetActivate%20For))
  (bind _returnvalue (Actor|GetComponentbyClass _activate_for "/Script/Engine.CharacterMovementComponent"))
  (Utilities|IsValid _activate_for
    (:Is%20Valid
      (Variables|/Script/Engine.CharacterMovementComponent|SetMaxWalkSpeed _returnvalue (/ (Class|MovementComponent|GetMaxSpeed _returnvalue) 1e+01)))
    (:Is%20Not%20Valid
      _))
  (|CallParentFunction))

(event EventOnActivated
  (params (ActivateFor :type Actor%20Object%20Reference))
  (bind _returnvalue (Actor|GetComponentbyClass ActivateFor "/Script/Engine.CharacterMovementComponent"))
  (Variables|Default|SetActivate%20For ActivateFor)
  (Variables|/Script/Engine.CharacterMovementComponent|SetMaxWalkSpeed _returnvalue (* (Class|MovementComponent|GetMaxSpeed _returnvalue) 1e+01)))

(fn ConstructionScript)